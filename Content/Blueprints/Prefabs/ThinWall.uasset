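; ThinWall is a prefab that builds a framed thin wall, plain or glass, sized by the Finish vector.
; The construction script places four rotated, stretched frame meshes from the origin and Finish corners, then adds a wall mesh scaled to the same X and Z.
; A dynamic instance of either grid glass or plain material receives the color and size-scaled UV tiling.
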(fn `UserConstructionScript`
  (bind (_x _y) (`KismetMathLibrary.BreakVector2D` (`self.UVMultiplier`)))
  (bind _x_2 (.x (/ (`self.Finish`) 10.0)))
  (bind _z (.z (/ (`self.Finish`) 10.0)))
  (`|ExecutionSequence`
    (:`then_0`
      ;[1 1 1] Frame
      (for _index (range 4)
        (bind _returnvalue (`AddComponent|NODE_AddStaticMeshComponent-0` :`RelativeTransform` (`KismetMathLibrary.MakeTransform` (`KismetMathLibrary.SelectVector` (0.0 0.0 0.0) (`self.Finish`) (<= _index 1)) (select `int` _index :`0` (struct) :`1` (struct :`Pitch` 90.0) :`2` (struct :`Pitch` -90.0) :`3` (struct :`Pitch` 180.0) :!type "Rotator Structure") (`KismetMathLibrary.MakeVector` (select `int` _index :`0` _x_2 :`1` _z :`2` _z :`3` _x_2) 1.0 1.0))))
        (`StaticMeshComponent.SetStaticMesh` _returnvalue "/Game/Assets/Models/ThinWall/ThinWallFrame.ThinWallFrame")))
    (:`then_1`
      ;[1 1 1] Wall Generation
      (bind _returnvalue_2 (`AddComponent|NODE_AddStaticMeshComponent-1` :`RelativeTransform` (`KismetMathLibrary.MakeTransform` (0.0 0.0 0.0) (struct) (`KismetMathLibrary.MakeVector` (.x (/ (`self.Finish`) 10.0)) 1.0 (.z (/ (`self.Finish`) 10.0))))))
      (`StaticMeshComponent.SetStaticMesh` _returnvalue_2 "/Game/Assets/Models/ThinWall/ThinWall.ThinWall")
      (bind _returnvalue_3 (`PrimitiveComponent.CreateDynamicMaterialInstance` _returnvalue_2 0 (select `bool` (`self.Glass`) :`false` "/Game/Assets/Materials/M_PlainMat.M_PlainMat" :`true` "/Game/Assets/Materials/M_GridGlass.M_GridGlass" :!type "MaterialInterface Object Reference")))
      (`|ExecutionSequence`
        (:`then_0`
          ;[1 1 1] UV
          (`MaterialInstanceDynamic.SetScalarParameterValue` _returnvalue_3 "U" (* (.x (/ (`self.Finish`) 10.0)) _x))
          (`MaterialInstanceDynamic.SetScalarParameterValue` _returnvalue_3 "V" (* (.z (/ (`self.Finish`) 10.0)) _y)))
        (:`then_1`
          (`MaterialInstanceDynamic.SetVectorParameterValue` _returnvalue_3 "Color" (`self.Color`)))))))