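; Firearm Blueprint, extending a parent weapon, that handles shooting, ammo and reloading for player characters.
; On authority, Shoot spawns FireProjectile if set or applies line-trace damage, then auto-reloads when empty; remote use plays effects.
; Spread comes from a random stream; effects add recoil, muzzle flash, and hitscan trails and decals from their own trace.
; The Reloading RepNotify runs a timer that moves reserve ammo into the magazine.
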(event `FromClientReloadWeapon`
  (if (`self.AbleToReload`)
    (`self.ServerReloadWeapon`)
    (`self.ReloadWeapon`)))

(event `ServerReloadWeapon`
  (if (`self.AbleToReload`)
    (`self.ReloadWeapon`)))

(event `self.PlayWeaponEffects`
  (bind _returnvalue_location (`KismetMathLibrary.BreakTransform` (`SceneComponent.GetSocketTransform` (`self.WeaponMesh`) "Sk_GunFire" "RTS_World")))
  (`parent.PlayWeaponEffects`)
  (`|ExecutionSequence`
    (:`then_0`
      (if (not (`self.IsOtherPlayer`))
        (bind (_direction _erp) (`Timeline|Test` :!via `PlayFromStart`)
          (:`Update`
            (`Pawn.AddControllerPitchInput` (`self.WeaponOwner`) (* _erp (`self.Recoil`) -1.0))))))
    (:`then_1`
      (`GameplayStatics.SpawnEmitterAttached` "/Game/Assets/StarterContent/Particles/P_GunFlash.P_GunFlash" (`self.WeaponMesh`) "Sk_GunFire" (0.0 0.0 0.0) (struct) (0.1 0.1 0.1) "SnapToTargetIncludingScale"))
    (:`then_2`
      (`|ExecutionSequence`
        (:`then_0`
          (if (not (`KismetSystemLibrary.IsValidClass` (`self.FireProjectile`)))
            (bind _asbp_player_character (cast `/Game/Blueprints/Player/BP_PlayerCharacter` (`self.GetInstigator`)))
            (bind _returnvalue (`SceneComponent.K2_GetComponentLocation` (`/Game/Blueprints/Player/BP_PlayerCharacter.Camera` _asbp_player_character)))
            (bind (_outhit _returnvalue_2) (`KismetSystemLibrary.LineTraceSingleForObjects` _returnvalue (+ _returnvalue (* (`self.GetShootDirection`) 10000.0)) (`|MakeArray` "ObjectTypeQuery1" "ObjectTypeQuery2" "ObjectTypeQuery3" :!type "EObjectTypeQuery Enum") false (`|MakeArray` self (`self.GetInstigator`) :!type "Actor Object Reference")))
            (bind (_bblockinghit _binitialoverlap _time _distance _location _impactpoint _normal _impactnormal _physmat _hitactor _hitcomponent _hitbonename _hititem _faceindex _tracestart _traceend) (`GameplayStatics.BreakHitResult` _outhit))
            (bind _returnvalue_3 (`|SpawnActorFromClass` "/Game/Blueprints/Weapons/Other/BP_WeaponTrail.BP_WeaponTrail_C" (`KismetMathLibrary.MakeTransform` _returnvalue_location (`KismetMathLibrary.FindLookAtRotation` _returnvalue_location (`KismetMathLibrary.SelectVector` _location _traceend _bblockinghit))) "Undefined" "OverrideRootScale" null _outhit null))
            (`self.SetLifeSpan` _returnvalue_3 0.05)
            (if _returnvalue_2
              (`self.HoleMaterial`
                (:`then`
                  (bind (_bblockinghit_2 _binitialoverlap_2 _time_2 _distance_2 _location_2 _impactpoint_2 _normal_2) (`GameplayStatics.BreakHitResult` _outhit))
                  (bind _returnvalue_4 (`|SpawnActorFromClass` "/Script/Engine.DecalActor" (`KismetMathLibrary.MakeTransform` _location_2 (struct) (0.01 0.01 0.01)) "AlwaysSpawn" "OverrideRootScale" null null))
                  (`self.SetLifeSpan` _returnvalue_4 30.0)
                  (`self.K2_SetActorRotation` _returnvalue_4 (`KismetMathLibrary.Conv_VectorToRotator` (* _normal_2 -1.0)) false)
                  (bind _decal (`DecalActor.Decal` _returnvalue_4))
                  (`DecalComponent.SetDecalMaterial` _decal (`self.HoleMaterial`))
                  (`DecalComponent.SetFadeScreenSize` _decal 1e-05))
                (:`else`)))))))))

(fn `AbleToReload`
  (returns (ReturnValue :type Boolean))
  (return (and (!= (`.CurrentAmmo` (defaults `/Game/Blueprints/Weapons/BP_FireWeapons` (`GameplayStatics.GetObjectClass` self))) (`self.CurrentAmmo`)) (> (`self.TotalAmmo`) 0) (not (`KismetSystemLibrary.K2_IsValidTimerHandle` (`self.ReloadTimer`))))))

(fn `AbleToUseWeapon`
  (returns (Out :type Boolean))
  (return (and (`parent.AbleToUseWeapon`) (not (`self.Reloading`)))))

(fn `FinishReload`
  (set `self.Reloading` false)
  (set `self.CurrentAmmo` (+ (`self.CurrentAmmo`) (`self.AmmoToReload`)))
  (set `self.TotalAmmo` (- (`self.TotalAmmo`) (`self.AmmoToReload`))))

(fn `GetReaminingReloadTime`
  (returns (Out :type "Float (double-precision)"))
  (return (`KismetSystemLibrary.K2_GetTimerRemainingTimeHandle` (`self.ReloadTimer`))))

(fn `GetShootDirection`
  (returns (ReturnValue :type "Vector Structure"))
  (locals (NewLocalVar_0 :type "Float (double-precision)" :default 0.0))
  (bind _spreadangle (`self.SpreadAngle`))
  (bind _weaponowner (`self.WeaponOwner`))
  (bind _spreadangle_2 (`self.SpreadAngle`))
  (bind _returnvalue (`KismetMathLibrary.RotateAngleAxis` (`self.GetActorForwardVector` _weaponowner) (* (`/Game/Blueprints/Player/BP_PlayerCharacter.LookVerticalAngle` _weaponowner) -1.0) (`self.GetActorRightVector` _weaponowner)))
  (bind _returnvalue_2 (`KismetMathLibrary.Conv_VectorToRotator` _returnvalue))
  (return (`KismetMathLibrary.RotateAngleAxis` (`KismetMathLibrary.RotateAngleAxis` _returnvalue (`KismetMathLibrary.RandomFloatInRangeFromStream` (* _spreadangle_2 -1.0) _spreadangle_2 (`self.RandomStream`)) (`KismetMathLibrary.GetRightVector` _returnvalue_2)) (`KismetMathLibrary.RandomFloatInRangeFromStream` (* _spreadangle -1.0) _spreadangle (`self.RandomStream`)) (`KismetMathLibrary.GetUpVector` _returnvalue_2))))

(fn `OnRep_Reloading`
  (if (`self.Reloading`)
    (`|ExecutionSequence`
      (:`then_0`
        (if (not (`self.IsOtherPlayer`))
          (bind _returnvalue (`KismetSystemLibrary.K2_SetTimer` null "FinishReload" (`self.ReloadTime`)))
          (set `self.ReloadTimer` _returnvalue)
          (set `self.AmmoToReload` (`KismetMathLibrary.Min` (- (`.CurrentAmmo` (defaults `/Game/Blueprints/Weapons/BP_FireWeapons` (`GameplayStatics.GetObjectClass` self))) (`self.CurrentAmmo`)) (`self.TotalAmmo`)))))
      (:`then_1`
        (`self.ReloadStarted`)))
    (else
      (`KismetSystemLibrary.K2_ClearAndInvalidateTimerHandle` (`self.ReloadTimer`))
      (`self.ReloadFinished`))))

(fn `ReloadWeapon`
  (if (not (`self.Reloading`))
    (set `self.Reloading` true)))

(fn `ShootFireTrace`
  (locals (L_Direction :type "Vector Structure" :default (0.0 0.0 0.0)))
  (bind _asbp_player_character (cast `/Game/Blueprints/Player/BP_PlayerCharacter` (`self.GetInstigator`))
    (:`then`
      (set `local.L_Direction` (`self.GetShootDirection`))
      (bind _returnvalue (`SceneComponent.K2_GetComponentLocation` (`/Game/Blueprints/Player/BP_PlayerCharacter.Camera` _asbp_player_character)))
      (bind _outhit (`KismetSystemLibrary.LineTraceSingleForObjects` _returnvalue (+ _returnvalue (* (`local.L_Direction`) 10000.0)) (`|MakeArray` "ObjectTypeQuery1" "ObjectTypeQuery2" "ObjectTypeQuery3" :!type "EObjectTypeQuery Enum") false (`|MakeArray` self (`self.GetInstigator`) :!type "Actor Object Reference")))
      (bind (_bblockinghit _binitialoverlap _time _distance _location _impactpoint _normal _impactnormal _physmat _hitactor _hitcomponent _hitbonename _hititem _faceindex _tracestart _traceend) (`GameplayStatics.BreakHitResult` _outhit))
      (bind _returnvalue_2 (`GameplayStatics.ApplyPointDamage` _hitactor (`self.Damage`) (`KismetMathLibrary.GetDirectionUnitVector` _traceend _tracestart) _outhit (`self.GetInstigatorController`) self))
      (`self.OnWeaponDamagedActor` _returnvalue_2 _hitactor)
      (return))
    (:`CastFailed`
      (return))))

(fn `SpawnShootProjectile`
  (locals (L_ShootDirection :type "Vector Structure" :default (0.0 0.0 0.0)))
  (bind _weaponowner (`self.WeaponOwner`))
  (set `local.L_ShootDirection` (`self.GetShootDirection`))
  (`|SpawnActorFromClass` (`self.FireProjectile`) (`KismetMathLibrary.MakeTransform` (+ (`SceneComponent.K2_GetComponentLocation` (`/Game/Blueprints/Player/BP_PlayerCharacter.Camera` _weaponowner)) (* (`self.GetActorForwardVector` (`Pawn.GetController` _weaponowner)) 70.0)) (`KismetMathLibrary.Conv_VectorToRotator` (`local.L_ShootDirection`))) "AlwaysSpawn" "OverrideRootScale" self (`self.Damage`) self (`self.GetInstigator`)))

(fn `UserConstructionScript`
  (`parent.UserConstructionScript`))

(fn `UseWeapon`
  (returns (Used :type Boolean))
  (bind _used (`parent.UseWeapon`))
  (if _used
    (`|ExecutionSequence`
      (:`then_0`
        (`/Engine/EditorBlueprintResources/ActorMacros.Switch Has Authority`
          (:`Authority`
            (`|ExecutionSequence`
              (:`then_0`
                (if (`KismetSystemLibrary.IsValidClass` (`self.FireProjectile`))
                  (`self.SpawnShootProjectile`)
                  (else
                    (`self.ShootFireTrace`))))
              (:`then_1`
                (if (and (<= (`self.CurrentAmmo`) 0) (> (`self.TotalAmmo`) 0))
                  (`self.ReloadWeapon`)))))
          (:`Remote`
            (`self.PlayWeaponEffects`)
            (return true))))
      (:`then_1`
        (return true)))
    (else
      (return false))))