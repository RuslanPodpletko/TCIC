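; Hitscan weapon projectile that deals instant point damage along a line instead of travelling.
; On BeginPlay it casts its instigator to BP_PlayerCharacter and traces from that camera's location along the projectile's forward vector, ignoring both actors, with debug drawing on.
; It applies Damage to the hit actor, credited to the instigator's controller, then destroys itself.
; A failed cast skips everything, including the destroy.
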(event `self.ReceiveBeginPlay`
  (bind _asbp_player_character (cast `/Game/Blueprints/Player/BP_PlayerCharacter` (`self.GetInstigator`)))
  (bind _returnvalue (`SceneComponent.K2_GetComponentLocation` (`/Game/Blueprints/Player/BP_PlayerCharacter.Camera` _asbp_player_character)))
  (bind _outhit (`KismetSystemLibrary.LineTraceSingleForObjects` _returnvalue (+ _returnvalue (* (`self.GetActorForwardVector`) 10000.0)) (`|MakeArray` "ObjectTypeQuery1" "ObjectTypeQuery2" "ObjectTypeQuery3" :!type "EObjectTypeQuery Enum") false (`|MakeArray` self (`self.GetInstigator`) :!type "Actor Object Reference") "ForDuration"))
  (bind (_bblockinghit _binitialoverlap _time _distance _location _impactpoint _normal _impactnormal _physmat _hitactor _hitcomponent _hitbonename _hititem _faceindex _tracestart _traceend) (`GameplayStatics.BreakHitResult` _outhit))
  (`GameplayStatics.ApplyPointDamage` _hitactor (`self.Damage`) (`KismetMathLibrary.GetDirectionUnitVector` _traceend _tracestart) _outhit (`self.GetInstigatorController`) self)
  (`self.K2_DestroyActor`))

(fn `UserConstructionScript`
  (`parent.UserConstructionScript`))