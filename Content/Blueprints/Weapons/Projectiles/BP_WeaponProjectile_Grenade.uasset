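; Grenade projectile that the server throws with a forward impulse and random spin, then detonates after a timed delay.
; Explode sets the replicated Exploded flag, applies full radial damage, notifies the owning weapon and sets a short lifespan.
; OnRep_Exploded freezes and hides the grenade, spawning explosion particles and sound only on remotes.
; A disconnected gamemode-based ignore trace remains unused; its note defers that filtering to the health component.
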(event `self.ReceiveBeginPlay`
  (`/Engine/EditorBlueprintResources/ActorMacros.Switch Has Authority`
    (:`Authority`
      (`PrimitiveComponent.AddImpulse` (`self.Box`) (* (`self.GetActorForwardVector`) (`self.ThrowPower`)) "None" false)
      (`PrimitiveComponent.AddAngularImpulseInRadians` (`self.Box`) (`KismetMathLibrary.MakeVector` (`KismetMathLibrary.RandomFloatInRange` -500.0 500.0) (`KismetMathLibrary.RandomFloatInRange` -500.0 500.0) (`KismetMathLibrary.RandomFloatInRange` -500.0 500.0)) "None" false)
      (`KismetSystemLibrary.K2_SetTimer` null "Explode" (`self.ExplotionDelay`)))))

(fn `Explode`
  (locals (L_Ignore :type "Array of Actor Object Reference"))
  (set `self.Exploded` true)
  (`GameplayStatics.ApplyRadialDamage` :`BaseDamage` (`self.Damage`) :`Origin` (`self.K2_GetActorLocation`) :`DamageRadius` (`self.ExplosionRadius`) :`DamageCauser` self :`InstigatedByController` (`self.GetInstigatorController`) :`bDoFullDamage` true :`DamagePreventionChannel` "ECC_WorldStatic")
  (`/Game/Blueprints/Weapons/BP_WEapon.OnWeaponDamagedActor` (`self.Weapon`) (`self.Damage`) null)
  (`self.SetLifeSpan` 5.0))

(fn `HideGrenade`
  (`PrimitiveComponent.SetSimulatePhysics` (`self.Box`) false)
  (`self.SetActorEnableCollision` false)
  (`ActorComponent.K2_DestroyComponent` (`self.StaticMesh`))
  (`ActorComponent.K2_DestroyComponent` (`self.StaticMesh1`)))

(fn `OnRep_Exploded`
  (`self.HideGrenade`)
  (`/Engine/EditorBlueprintResources/ActorMacros.Switch Has Authority`
    (:`Remote`
      (`GameplayStatics.SpawnEmitterAtLocation` "/Game/Assets/StarterContent/Particles/P_Explosion.P_Explosion" (`self.K2_GetActorLocation`))
      (`GameplayStatics.PlaySoundAtLocation` "/Game/Assets/Sounds/335152__apenguin73__explosion-test.335152__apenguin73__explosion-test" (`self.K2_GetActorLocation`) (struct) 1.0 1.0 0.0 "/Game/Assets/Sounds/SA_Shot.SA_Shot"))))

(fn `UserConstructionScript`
  (`parent.UserConstructionScript`))