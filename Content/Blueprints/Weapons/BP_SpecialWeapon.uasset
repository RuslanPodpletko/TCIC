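; Weapon Blueprint for placing a "special" actor in the world, with a placement preview.
; On the owning remote client, Tick moves a collisionless ghost to the camera trace hit, tinting it by box-overlap and distance checks.
; Use input passes through only when that placement is valid.
; The server spawns the real actor from its own shorter controller-direction trace, independent of the ghost, and drops the weapon when ammo runs out.
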(event `self.ReceiveTick`
  (params (DeltaSeconds :type "Float (single-precision)"))
  (bind _specialbeforeset (`self.SpecialBeforeSet`))
  (bind _camera (`/Game/Blueprints/Player/BP_PlayerCharacter.Camera` (`self.WeaponOwner`)))
  (bind _collision (`/Game/Blueprints/Weapons/Specials/BP_Special.Collision` (`self.SpecialBeforeSet`)))
  (bind _returnvalue (`SceneComponent.K2_GetComponentLocation` _camera))
  (bind _returnvalue_2 (`SceneComponent.K2_GetComponentLocation` _collision))
  (`parent.ReceiveTick` DeltaSeconds)
  (`/Engine/EditorBlueprintResources/ActorMacros.Switch Has Authority`
    (:`Remote`
      (bind _weaponowner (`self.WeaponOwner`)
        (:`then`
          (if (`Pawn.IsLocallyControlled` _weaponowner)
            (if (== (`/Game/Blueprints/Components/Player/BP_WeaponManager.CurrentWeapon` (`/Game/Blueprints/Player/BP_PlayerCharacter.BP_WeaponManager` (`self.WeaponOwner`))) self)
              (`self.SpecialBeforeSet`
                (:`then`
                  (bind _outhit (`KismetSystemLibrary.LineTraceSingle` _returnvalue (+ _returnvalue (* (`SceneComponent.GetForwardVector` _camera) 9999.0)) "TraceTypeQuery1" false (`|MakeArray` (`self.WeaponOwner`) (`self.SpecialBeforeSet`) :!type "Actor Object Reference")))
                  (bind (_bblockinghit _binitialoverlap _time _distance _location _impactpoint _normal _impactnormal _physmat _hitactor _hitcomponent _hitbonename _hititem _faceindex _tracestart) (`GameplayStatics.BreakHitResult` _outhit))
                  (if _bblockinghit
                    (`self.K2_SetActorTransform` (`self.SpecialBeforeSet`) (`KismetMathLibrary.MakeTransform` _location (`KismetMathLibrary.Conv_VectorToRotator` (`self.GetActorForwardVector` (`self.WeaponOwner`)))) false false)
                    (bind (_outhit_2 _returnvalue_3) (`KismetSystemLibrary.BoxTraceSingleForObjects` _returnvalue_2 _returnvalue_2 (`BoxComponent.GetScaledBoxExtent` _collision) (`SceneComponent.K2_GetComponentRotation` _collision) (`|MakeArray` "ObjectTypeQuery1" "ObjectTypeQuery2" "ObjectTypeQuery3" :!type "EObjectTypeQuery Enum") false (`|MakeArray` _specialbeforeset :!type "Actor Object Reference")))
                    (set `self.CanSetSpecial` (not (or _returnvalue_3 (> (`KismetMathLibrary.VSize` (- (`self.K2_GetActorLocation` _specialbeforeset) _tracestart)) (`self.SetMaxDistance`)))))
                    (`MaterialInstanceDynamic.SetVectorParameterValue` (`self.BeforeSetDynamMaterials`) "Color" (`KismetMathLibrary.SelectColor` (struct :`R` 1.0 :`G` 1.0 :`B` 1.0 :`A` 1.0) (struct :`R` 1.0 :`G` 0.034709 :`A` 1.0) (`self.CanSetSpecial`)))
                    (else
                      (`self.K2_DestroyActor` (`self.SpecialBeforeSet`)))))
                (:`else`
                  (bind _returnvalue_4 (`|SpawnActorFromClass` (`self.SpecialClass`) (`KismetMathLibrary.MakeTransform` (0.0 0.0 0.0)) "AlwaysSpawn" "OverrideRootScale" null 0.0 null))
                  (bind _output_get (set `self.SpecialBeforeSet` _returnvalue_4))
                  (`self.SetActorEnableCollision` _output_get false)
                  (for _array_element (`self.K2_GetComponentsByClass` _output_get "/Script/Engine.MeshComponent")
                    (bind _returnvalue_5 (`PrimitiveComponent.CreateDynamicMaterialInstance` _array_element 0 "/Game/Assets/Weapons/Specials/M_SpecialBeforeSet.M_SpecialBeforeSet"))
                    (`KismetArrayLibrary.Array_Add` (`self.BeforeSetDynamMaterials`) _returnvalue_5))))
              (else
                (bind _specialbeforeset_2 (`self.SpecialBeforeSet`)
                  (:`then`
                    (`self.K2_DestroyActor` _specialbeforeset_2))
                  (:`else`))))))
        (:`else`)))))

(event `self.ReceiveDestroyed`
  (`parent.ReceiveDestroyed`)
  (`/Engine/EditorBlueprintResources/ActorMacros.Switch Has Authority`
    (:`Remote`
      (bind _specialbeforeset (`self.SpecialBeforeSet`)
        (:`then`
          (`self.K2_DestroyActor` _specialbeforeset))
        (:`else`)))))

(event `self.FromClientToggleUseWeapon`
  (params (Use :type Boolean))
  (if Use
    (if (`self.CanSetSpecial`)
      (`parent.FromClientToggleUseWeapon` true))
    (else
      (`parent.FromClientToggleUseWeapon` false))))

(event `self.OnWeaponDropped`
  (bind _specialbeforeset (`self.SpecialBeforeSet`)
    (:`then`
      (`self.K2_DestroyActor` _specialbeforeset))
    (:`else`)))

(fn `SetSpecial`
  (bind _weaponowner (`self.WeaponOwner`))
  (bind _returnvalue (+ (`self.K2_GetActorLocation` _weaponowner) (0.0 0.0 50.0)))
  (bind _outhit (`KismetSystemLibrary.LineTraceSingle` _returnvalue (+ _returnvalue (* (`self.GetActorForwardVector` (`Pawn.GetController` _weaponowner)) 500.0)) "TraceTypeQuery1"))
  (`|SpawnActorFromClass` (`self.SpecialClass`) (`KismetMathLibrary.MakeTransform` (`.Location` (`GameplayStatics.BreakHitResult` _outhit)) (`self.K2_GetActorRotation` (`self.WeaponOwner`))) "AlwaysSpawn" "OverrideRootScale" self (`self.Damage`) (`self.GetInstigator`)))

(fn `UserConstructionScript`
  (`parent.UserConstructionScript`))

(fn `UseWeapon`
  (returns (Used :type Boolean))
  (bind _used (`parent.UseWeapon`))
  (if _used
    (`/Engine/EditorBlueprintResources/ActorMacros.Switch Has Authority`
      (:`Authority`
        (`self.SetSpecial`)
        (if (<= (`self.CurrentAmmo`) 0)
          (`/Game/Blueprints/Components/Player/BP_WeaponManager.DropWeapon` (`/Game/Blueprints/Player/BP_PlayerCharacter.BP_WeaponManager` (`self.WeaponOwner`)) self)
          (return true))))
    (else
      (return false))))