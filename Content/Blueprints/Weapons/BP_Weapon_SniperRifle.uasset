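; Sniper rifle weapon Blueprint whose secondary action aims through a scope.
; While the secondary action is active, spread drops to zero and, for a local player controller, the owner's camera FOV narrows and a lazily created, reused scope widget is shown.
; Stopping restores spread from the class defaults and, for the local player, sets a wider FOV and removes the overlay.
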(event `self.UseSecondaryAction`
  (`parent.UseSecondaryAction`)
  (if (`self.UsingSecondary`)
    (set `self.SpreadAngle` 0.0)
    (if (`Controller.IsLocalPlayerController` (`self.GetInstigatorController`))
      (`CameraComponent.SetFieldOfView` (`/Game/Blueprints/Player/BP_PlayerCharacter.Camera` (`self.WeaponOwner`)) 15.0)
      (`self.SniperScope`
        (:`then`
          _)
        (:`else`
          (bind _returnvalue (`|CreateWidget` "/Game/UI/Other/SniperScope/W_SniperScope.W_SniperScope_C"))
          (bind _output_get (set `self.SniperScope` _returnvalue))))
      (`UserWidget.AddToViewport` _output_get -1))))

(event `self.StopUseSecondaryAction`
  (`parent.StopUseSecondaryAction`)
  (set `self.SpreadAngle` (defaults `/Game/Blueprints/Weapons/BP_Weapon_SniperRifle` (`GameplayStatics.GetObjectClass` self)))
  (if (`Controller.IsLocalPlayerController` (`self.GetInstigatorController`))
    (`CameraComponent.SetFieldOfView` (`/Game/Blueprints/Player/BP_PlayerCharacter.Camera` (`self.WeaponOwner`)) 90.0)
    (`Widget.RemoveFromParent` (`self.SniperScope`))))

(fn `UserConstructionScript`
  (`parent.UserConstructionScript`))