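; Player camera manager that shows a directional damage indicator and camera shake when the player's character takes damage.
; After a short startup delay it listens for possession, then binds to the character's health component and adds a dynamic damage post-process material to its camera.
; Each hit converts the damage vector into character-relative direction for the material and resets a lerp parameter, which Tick fades to zero.
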(event `self.ReceiveBeginPlay`
  (`KismetSystemLibrary.Delay` 1.0)
  (bind _asbp_player_controller (cast `/Game/Blueprints/Player/BP_PlayerController` (`self.GetOwner`)))
  (add `/Game/Blueprints/Player/BP_PlayerController.PossesedToCharacter` _asbp_player_controller (delegate `PossesedToCharacter`)))

(event `PossesedToCharacter`
  (params (Char :type "/Game/Blueprints/Player/BP_PlayerCharacter Object Reference"))
  (bind _output_get (set `self.CurrentCharacter` Char))
  (add `/Game/Blueprints/Components/Player/BP_HealthComponent.ClientDamageRecieved` (`/Game/Blueprints/Player/BP_PlayerCharacter.BP_HealthComponent` _output_get) (delegate `ClientDamageRecieved`))
  (bind _returnvalue (`KismetMaterialLibrary.CreateDynamicMaterialInstance` "/Game/Assets/Other/PostProcess/DamagePP/M_PP_DamageNotify.M_PP_DamageNotify"))
  (bind _output_get_2 (set `self.DamageMaterial` _returnvalue))
  (`CameraComponent.AddOrUpdateBlendable` (`/Game/Blueprints/Player/BP_PlayerCharacter.Camera` (`self.CurrentCharacter`)) _output_get_2 1.0))

(event `ClientDamageRecieved`
  (params (Damage :type "Float (double-precision)") (DamageVector :type "Vector Structure"))
  (bind (_returnvalue_x _returnvalue_y) (`KismetMathLibrary.BreakVector` (`KismetMathLibrary.Normal` (`KismetMathLibrary.LessLess_VectorRotator` DamageVector (`KismetMathLibrary.ComposeRotators` (`self.K2_GetActorRotation` (`self.CurrentCharacter`)) (struct :`Yaw` 90.0))))))
  (set `self.DamageLerp` 1.0)
  (set `self.ShowingDamage` true)
  (`MaterialInstanceDynamic.SetVectorParameterValue` (`self.DamageMaterial`) "Direction" (make `LinearColor` _returnvalue_x _returnvalue_y))
  (`self.PlayCameraShake` "/Game/Blueprints/Player/Camera/CamShake_Damage.CamShake_Damage_C"))

(event `self.ReceiveTick`
  (params (DeltaSeconds :type "Float (single-precision)"))
  (if (`self.ShowingDamage`)
    (set `self.DamageLerp` (`KismetMathLibrary.FInterpTo_Constant` (`self.DamageLerp`) 0.0 (`GameplayStatics.GetWorldDeltaSeconds`) 5.0))
    (`MaterialInstanceDynamic.SetScalarParameterValue` (`self.DamageMaterial`) "Lerp" (`self.DamageLerp`))
    (if (<= (`self.DamageLerp`) 0.0)
      (set `self.ShowingDamage` false))))

(fn `UserConstructionScript`)