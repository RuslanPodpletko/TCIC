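; Map vote controller component that runs a timed vote on the next map, picking random unique candidates from DT_VoteMaps.
; StartVote enables Tick, which decrements the timer and stops the vote at zero.
; SetVote stores choices by PlayerArray index and recomputes the leader, breaking ties randomly.
; RepNotifies on Maps and VoteInProgress fire events for generated candidates, vote start, and vote end with the winning map.
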(event `self.ReceiveTick`
  (params (DeltaSeconds :type "Float (single-precision)"))
  (bind _result (`/Engine/EditorBlueprintResources/StandardMacros.DecrementInt` (`self.MapVoteTime`))
    (:`  `
      (if (<= _result 0)
        (`self.StopVote`)))))

(fn `ChooseMapsToVote`
  (locals (L_Maps :type "Array of Name") (L_RandomMapIndex :type Integer :default 0))
  (bind _outrownames (`DataTableFunctionLibrary.GetDataTableRowNames` "/Game/Data/DataTables/DT_VoteMaps.DT_VoteMaps"))
  (set `local.L_Maps` _outrownames)
  (for _ (range 1 (+ (`self.NumberOfMaps`) 1))
    (if (> (`KismetArrayLibrary.Array_Length` (`local.L_Maps`)) 0)
      (set `local.L_RandomMapIndex` (`KismetMathLibrary.RandomInteger` (`KismetArrayLibrary.Array_Length` (`local.L_Maps`))))
      (`KismetArrayLibrary.Array_Add` (`self.Maps`) (`|GetArrayItem` (`local.L_Maps`) (`local.L_RandomMapIndex`)))
      (`KismetArrayLibrary.Array_Remove` (`local.L_Maps`) (`local.L_RandomMapIndex`))
      (else
        (return))))
  (return))

(fn `GetMapVotes`
  (params (MapIndex :type Integer))
  (returns (Votes :type Integer))
  (locals (L_Votes :type Integer))
  (for _array_element (`self.PlayersVotes`)
    (if (== _array_element MapIndex)
      (`/Engine/EditorBlueprintResources/StandardMacros.IncrementInt` (`local.L_Votes`))))
  (return (`local.L_Votes`)))

(fn `GetMaxVotesMap`
  (returns (MapName :type Name))
  (return (`|GetArrayItem` (`self.Maps`) (`self.MaxVotesMap`))))

(fn `GetVotedMap`
  (returns (MapIndex :type Integer))
  (locals (L_MaxVotesIndexes :type "Array of Integer") (L_Votes :type "Array of Integer"))
  (bind _l_maxvotesindexes (`local.L_MaxVotesIndexes`))
  (for (_ _array_index) (`self.Maps`)
    (`KismetArrayLibrary.Array_Add` (`local.L_Votes`) (`self.GetMapVotes` _array_index)))
  (`KismetArrayLibrary.Array_Add` (`local.L_MaxVotesIndexes`) (`KismetMathLibrary.MaxOfIntArray` (`local.L_Votes`)))
  (for (_array_element _array_index_2) (`local.L_Votes`)
    (if (and (== _array_element (`|GetArrayItem` (`local.L_Votes`) (`|GetArrayItem` (`local.L_MaxVotesIndexes`)))) (!= _array_index_2 (`|GetArrayItem` (`local.L_MaxVotesIndexes`))))
      (`KismetArrayLibrary.Array_Add` (`local.L_MaxVotesIndexes`) _array_index_2)))
  (return (`|GetArrayItem` _l_maxvotesindexes (`KismetMathLibrary.RandomInteger` (`KismetArrayLibrary.Array_Length` _l_maxvotesindexes)))))

(fn `OnRep_Maps`
  (`self.MapToVoteGenerated` (`self.Maps`)))

(fn `OnRep_VoteInProgress`
  (if (`self.VoteInProgress`)
    (`self.VoteStarted`)
    (else
      (`self.VoteEnded` (`self.GetMaxVotesMap`)))))

(fn `SetVote`
  (params (MapIndex :type Integer) (Player :type "/Game/Blueprints/Player/BP_PlayerState Object Reference"))
  (`KismetArrayLibrary.Array_Set` (`self.PlayersVotes`) (`KismetArrayLibrary.Array_Find` (`GameStateBase.PlayerArray` (`/Game/Blueprints/Libs/Funstions/BP_Functions_GlobalGetters.GetGameState`)) Player) MapIndex true)
  (set `self.MaxVotesMap` (`self.GetVotedMap`)))

(fn `StartVote`
  (`self.SetComponentTickEnabled` true)
  (`self.ChooseMapsToVote`)
  (set `self.VoteInProgress` true))

(fn `StopVote`
  (`self.SetComponentTickEnabled` false)
  (set `self.VoteInProgress` false))