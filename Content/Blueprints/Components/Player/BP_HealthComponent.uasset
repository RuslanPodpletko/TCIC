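; Player character component that tracks health, armor and stamina.
; The server handles damage the game mode allows, applies it to health and armor, broadcasts it with direction for point hits, and reports death to the game mode.
; Replicated Dead fires a death dispatcher through its RepNotify.
; Looping timers drain stamina while in use and moving, then regenerate it after a delay when usage stops or movement slows.
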(event Custom|OnPlayerTakeAnyDamage
  (params (DamagedActor :type Actor%20Object%20Reference) (Damage :type Float%20%28single-precision%29) (DamageType :type Damage%20Type%20Object%20Reference) (InstigatedBy :type Controller%20Object%20Reference) (DamageCauser :type Actor%20Object%20Reference))
  (if (CallFunction|ShouldbeDamaged InstigatedBy)
    (CallFunction|ApplyDamage Damage)
    (|Notifyanydamage Damage)
    (if (and (<= (Variables|Default|GetHealth) 0.0) (not (Variables|Default|GetDead)))
      (Variables|Default|SetDead true)
      (bind _asbp_base_gamemode (Utilities|Casting|CastToBP_BaseGamemode (Game|GetGameMode)))
      (Default|CharacterDead _asbp_base_gamemode (Variables|Default|GetCharacter) (.AsBP%20Player%20Controller (Utilities|Casting|CastToBP_PlayerController InstigatedBy)) DamageCauser))))

(event Custom|NotifyDamage
  (params (Damage :type Float%20%28single-precision%29) (DamageVector :type Vector))
  (Default|CallClientDamageRecieved Damage DamageVector))

(event Custom|OnPlayerTakePointDamage
  (params (DamagedActor :type Actor%20Object%20Reference) (Damage :type Float%20%28single-precision%29) (InstigatedBy :type Controller%20Object%20Reference) (HitLocation :type Vector) (FHitComponent :type Primitive%20Component%20Object%20Reference) (BoneName :type Name) (ShotFromDirection :type Vector) (DamageType :type Damage%20Type%20Object%20Reference) (DamageCauser :type Actor%20Object%20Reference))
  (if (CallFunction|ShouldbeDamaged InstigatedBy)
    (CallFunction|NotifyDamage Damage ShotFromDirection)
    (Variables|Default|SetDamageNotifyed true)))

(event EventBeginPlay
  (Variables|Default|SetHealth (Variables|Default|GetMaxHealth))
  (Variables|Default|SetArmor (Variables|Default|GetMaxArmor))
  (Variables|Stamina|SetStamina (Variables|Stamina|GetMaxStamina))
  (bind _asbp_player_character (Utilities|Casting|CastToBP_PlayerCharacter (Components|GetOwner)))
  (bind _output_get (Variables|Default|SetCharacter _asbp_player_character))
  (if (Networking|IsServer)
    (EventDispatchers|AssignOnTakeAnyDamage _output_get (EventDispatchers|CreateEvent :!event Custom|OnPlayerTakeAnyDamage))
    (EventDispatchers|AssignOnTakePointDamage (Variables|Default|GetCharacter) (EventDispatchers|CreateEvent :!event Custom|OnPlayerTakePointDamage))))

(fn ApplyDamage
  (params (Damage :type Float%20%28single-precision%29))
  (LocalVariables|SetL_Damage (|(Damage*(1-({1D373D31-4217-54E5-11C8-22AAAE895586}/200))) Damage))
  (Variables|Default|SetHealth (- (Variables|Default|GetHealth) (LocalVariables|GetL_Damage)))
  (Variables|Default|SetArmor (|(max(({1D373D31-4217-54E5-11C8-22AAAE895586}-({B285812E-4D8A-CBB1-6FA3-1FB3FEADE760}*2)),0)))))

(fn GetHealth
  (return (Variables|Default|GetHealth) (Variables|Default|GetMaxHealth)))

(fn GetArmor
  (return (Variables|Default|GetArmor) (Variables|Default|GetMaxArmor)))

(fn StartUsingStamina
  (bind _returnvalue (Utilities|Time|SetTimerbyFunctionName 0 "DecreaseStamina" (Variables|Stamina|GetStaminaChangeDelay) true))
  (Variables|Stamina|SetUseStaminaTimer _returnvalue)
  (Stamina|StopRegenerateStamina))

(fn DecreaseStamina
  (if (>= (Math|Vector|VectorLength (Variables|/Script/Engine.MovementComponent|GetVelocity (Variables|/Script/Engine.Character|GetCharacterMovement (Variables|Default|GetCharacter)))) 5e+01)
    (if (Utilities|Time|IsValidTimerHandle (Variables|Stamina|GetStartRegenTimer))
      (Stamina|StopRegenerateStamina))
    (bind _output_get (Variables|Stamina|SetStamina (Math|Float|Max(Float) 0.0 (- (Variables|Stamina|GetStamina) (* (Variables|Stamina|GetDecreaseStaminaSpeed) (Variables|Stamina|GetStaminaChangeDelay))))))
    (if (<= _output_get 0.0)
      (Stamina|StopUsingStamina)
      (Default|CallStaminaEnded))
    (elif (and (not (Utilities|Time|IsValidTimerHandle (Variables|Stamina|GetStartRegenTimer))) (not (Utilities|Time|IsValidTimerHandle (Variables|Stamina|GetStaminaRegenTimer))))
      (bind _returnvalue (Utilities|Time|SetTimerbyFunctionName 0 "StartRegenerateStamina" (Variables|Stamina|GetStartRegenStaminaDelay)))
      (Variables|Stamina|SetStartRegenTimer _returnvalue))))

(fn StopUsingStamina
  (Utilities|Time|ClearandInvalidateTimerbyHandle (Variables|Stamina|GetUseStaminaTimer))
  (bind _returnvalue (Utilities|Time|SetTimerbyFunctionName 0 "StartRegenerateStamina" (Variables|Stamina|GetStartRegenStaminaDelay)))
  (Variables|Stamina|SetStartRegenTimer _returnvalue))

(fn GetStamina
  (return (Variables|Stamina|GetStamina) (Variables|Stamina|GetMaxStamina)))

(fn StartRegenerateStamina
  (Utilities|Time|ClearandInvalidateTimerbyHandle (Variables|Stamina|GetStartRegenTimer))
  (bind _returnvalue (Utilities|Time|SetTimerbyFunctionName 0 "RegenerateStamina" (Variables|Stamina|GetStaminaChangeDelay) true))
  (Variables|Stamina|SetStaminaRegenTimer _returnvalue))

(fn RegenerateStamina
  (bind _output_get (Variables|Stamina|SetStamina (Math|Float|Min(Float) (+ (Variables|Stamina|GetStamina) (* (Variables|Stamina|GetRegenStaminaSpeed) (Variables|Stamina|GetStaminaChangeDelay))) (Variables|Stamina|GetMaxStamina))))
  (if (>= _output_get (Variables|Stamina|GetMaxStamina))
    (Stamina|StopRegenerateStamina)))

(fn StopRegenerateStamina
  (Utilities|Time|ClearandInvalidateTimerbyHandle (Variables|Stamina|GetStaminaRegenTimer))
  (Utilities|Time|ClearandInvalidateTimerbyHandle (Variables|Stamina|GetStartRegenTimer)))

(fn OnRepDead
  (Default|CallCharDead))

(fn ShouldbeDamaged
  (params (Object :type Object%20Object%20Reference))
  (if (not (Variables|Default|GetDead))
    (return (Default|ShouldDamagePlayer (CallFunction|GetGamemode) (CallFunction|GetCharactersController (Variables|Default|GetCharacter)) (.AsBP%20Player%20Controller (Utilities|Casting|CastToBP_PlayerController Object))))
    (else
      (return false))))